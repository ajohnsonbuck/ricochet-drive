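; BP_Reflector is a reflector actor that can be highlighted when selected.
; SelectItem and DeselectItem track an IsHighlighted flag and set the "ColorMultiplier" scalar parameter on the static mesh's materials to the highlighted or default value.
; SelectItem acts only when the reflector is not already highlighted, and BeginPlay calls DeselectItem to start in the default state.
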(event Collision|EventActorBeginOverlap
  (params (OtherActor :type Actor%20Object%20Reference))
  (|CallParentFunction OtherActor) ; This node is disabled and will not be called.\nDrag off pins to build functionality.
)

(event EventTick
  (params (DeltaSeconds :type Float%20%28single-precision%29))
  (|CallParentFunction DeltaSeconds) ; This node is disabled and will not be called.\nDrag off pins to build functionality.
)

(event EventSelectItem
  (if (not (Variables|Default|GetIsHighlighted?))
    (Variables|Default|SetIsHighlighted? true)
    (Rendering|Material|SetScalarParameterValueonMaterials (Variables|Default|GetStaticMeshComponent) "ColorMultiplier" (Variables|Default|GetHighlightedColorMultiplier))))

(event EventBeginPlay
  (CallFunction|DeselectItem))

(event EventDeselectItem
  (Variables|Default|SetIsHighlighted? false)
  (Rendering|Material|SetScalarParameterValueonMaterials (Variables|Default|GetStaticMeshComponent) "ColorMultiplier" (Variables|Default|GetDefaultColorMultiplier)))

(fn ConstructionScript
  (|CallParentFunction))