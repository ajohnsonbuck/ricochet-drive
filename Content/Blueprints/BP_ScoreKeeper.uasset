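; Score keeper actor that tracks hits, misses, combo and max combo, driving the score widget and BP_Thrusters.
; Each hit raises the combo and adds combo times base score; a miss resets it.
; Exact combo threshold matches pick text colors, and a color change triggers a tier sound and timeline text bounce.
; SummarizeScore fills the BP_ScoreCard widget with score, max combo and a threshold-based letter grade.
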(event Custom|Set%20Combo%20Color
  (params (Color :type Slate%20Color%20Structure))
  (bind _specifiedcolor (Utilities|Struct|BreakSlateColor Color))
  (bind _asbp_uiwidget (Utilities|Casting|CastToBP_UIWidget (UserInterface|GetWidget (Variables|/Game/Blueprints/BP_ScoreBox.BP_ScoreBox_C|GetWidget (Variables|Default|GetScoreBox)))))
  (Appearance|SetColorandOpacity (Variables|/Game/Blueprints/BP_UIWidget.BP_UIWidget_C|GetComboScoreText _asbp_uiwidget) Color :!class /Script/UMG.TextBlock)
  (if (not (== _specifiedcolor (Variables|Default|GetPreviousColor)))
    (CallFunction|PlayComboSound (Variables|Default|GetComboScore) (Variables|Default|GetComboThresholds) (Variables|Default|GetComboSounds))
    (CallFunction|BounceText))
  (Variables|Default|SetPreviousColor _specifiedcolor))

(event Custom|SetCombo
  (params (NewComboScore :type Integer))
  (if (> NewComboScore (Variables|Default|GetMaxCombo))
    (Variables|Default|SetMaxCombo NewComboScore))
  (bind _output_get (Variables|Default|SetComboScore NewComboScore))
  (bind _asbp_uiwidget (Utilities|Casting|CastToBP_UIWidget (UserInterface|GetWidget (Variables|/Game/Blueprints/BP_ScoreBox.BP_ScoreBox_C|GetWidget (Variables|Default|GetScoreBox)))))
  (Variables|/Script/UMG.TextBlock|SetText (Variables|/Game/Blueprints/BP_UIWidget.BP_UIWidget_C|GetComboScoreText _asbp_uiwidget) (Utilities|Text|ToText(String) (Utilities|String|ToString(Integer) _output_get)))
  (bind _textcolor (CallFunction|ChooseComboTextColor (Variables|Default|GetComboThresholds) (Variables|Default|GetComboColors)))
  (CallFunction|SetComboColor _textcolor)
  (bind _asbp_thrusters (Utilities|Casting|CastToBP_Thrusters (Variables|Default|GetThruster)))
  (Default|UpdateThrusters _asbp_thrusters _output_get))

(event Custom|Bounce%20Text
  (bind _asbp_uiwidget (Utilities|Casting|CastToBP_UIWidget (UserInterface|GetWidget (Variables|/Game/Blueprints/BP_ScoreBox.BP_ScoreBox_C|GetWidget (Variables|Default|GetScoreBox)))))
  (bind _textscale (Timeline|Text%20Bounce PlayFromStart)
    (:Update
      (Widget|Transform|SetRenderScale (Variables|/Game/Blueprints/BP_UIWidget.BP_UIWidget_C|GetComboScoreText _asbp_uiwidget) (Math|Conversions|ToVector2D(Vector) _textscale)))))

(event EventBeginPlay
  (bind _returnvalue (Actor|GetActorOfClass "/Game/Blueprints/BP_ScoreBox.BP_ScoreBox_C"))
  (Variables|Default|SetScoreBox _returnvalue)
  (Variables|Default|SetScore 0)
  (bind _returnvalue_2 (Actor|GetActorOfClass "/Game/Blueprints/BP_Thrusters.BP_Thrusters_C"))
  (Variables|Default|SetThruster _returnvalue_2))

(event EventSummarizeScore
  (bind _score (Variables|Default|GetScore))
  (bind _returnvalue (Actor|GetActorOfClass "/Game/Blueprints/BP_ScoreCard.BP_ScoreCard_C"))
  (bind _asbp_widget_score_card (Utilities|Casting|CastToBP_Widget_ScoreCard (UserInterface|GetWidget (Variables|/Game/Blueprints/BP_ScoreCard.BP_ScoreCard_C|GetScoreCard _returnvalue))))
  (Variables|/Script/UMG.TextBlock|SetText (Variables|/Game/Blueprints/BP_Widget_ScoreCard.BP_Widget_ScoreCard_C|GetScoreText _asbp_widget_score_card) (Utilities|Text|ToText(Integer) _score))
  (Variables|/Script/UMG.TextBlock|SetText (Variables|/Game/Blueprints/BP_Widget_ScoreCard.BP_Widget_ScoreCard_C|GetMaxComboText _asbp_widget_score_card) (Utilities|Text|ToText(Integer) (Variables|Default|GetMaxCombo)))
  (bind _gradetext (CallFunction|GetLetterGrade _score))
  (Variables|/Script/UMG.TextBlock|SetText (Variables|/Game/Blueprints/BP_Widget_ScoreCard.BP_Widget_ScoreCard_C|GetGradeText _asbp_widget_score_card) _gradetext))

(event EventResetCombo
  (CallFunction|SetCombo)
  (CallFunction|SetComboColor (Utilities|Struct|MakeSlateColor "(R=1.000000,G=0.008553,B=0.000000,A=1.000000)"))
  (Default|UpdateThrusters (Variables|Default|GetThruster)))

(event EventAddMiss
  (if (> (Variables|Default|GetComboScore) 0)
    (Audio|PlaySound2D "/Game/SFX/Miss.Miss" 2.0 1.0 0.0 0 0))
  (CallFunction|ResetCombo))

(event EventAddHit
  (bind _result (Math|Integer|IncrementInt (Variables|Default|GetComboScore))
    (:%20%20
      (CallFunction|SetCombo _result)
      (bind _newscore (CallFunction|CalculateScore _result (Variables|Default|GetScore) (Variables|Default|GetBaseHitScore)))
      (bind _output_get (Variables|Default|SetScore _newscore))
      (bind _asbp_uiwidget (Utilities|Casting|CastToBP_UIWidget (UserInterface|GetWidget (Variables|/Game/Blueprints/BP_ScoreBox.BP_ScoreBox_C|GetWidget (Variables|Default|GetScoreBox)))))
      (Variables|/Script/UMG.TextBlock|SetText (Variables|/Game/Blueprints/BP_UIWidget.BP_UIWidget_C|GetScoreText _asbp_uiwidget) (Utilities|Text|ToText(String) (Utilities|String|ToString(Integer) _output_get))))))

(fn ConstructionScript)

(fn CalculateScore
  (params (Combo%20Multiplier :type Integer) (Score :type Integer) (BaseHitScore :type Integer))
  (return (+ Score (* Combo%20Multiplier BaseHitScore))))

(fn GetLetterGrade
  (params (Score :type Integer))
  (bind _gradethresholds (Variables|Default|GetGradeThresholds))
  (if (>= Score (Utilities|Array|Get(acopy) _gradethresholds))
    (return "S")
    (elif (>= Score (Utilities|Array|Get(acopy) _gradethresholds 1))
      (return "A")
      (elif (>= Score (Utilities|Array|Get(acopy) _gradethresholds 2))
        (return "B")
        (elif true
          (return "C"))))))

(fn ChooseComboTextColor
  (params (ComboThresholds :type Array%20of%20Integers) (ComboColors :type Array%20of%20Slate%20Color%20Structures))
  (bind _comboscore (Variables|Default|GetComboScore))
  (bind _returnvalue (Utilities|Array|FindItem ComboThresholds _comboscore))
  (if (!= _returnvalue -1)
    (return (Utilities|Array|Get(acopy) ComboColors _returnvalue))
    (else
      (return (Utilities|Struct|MakeSlateColor (Variables|Default|GetPreviousColor))))))

(fn PlayComboSound
  (params (ComboScore :type Integer) (ComboThresholds :type Array%20of%20Integers) (ComboSounds :type Array%20of%20Sound%20Wave%20Object%20References))
  (Audio|PlaySound2D (Utilities|Array|Get(acopy) ComboSounds (Utilities|Array|FindItem ComboThresholds ComboScore)) 2.0 1.0 0.0 0 0))