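; BP_TargetSphere is a short-lived moving target that reacts visually when it passes through a BP_TargetStripe.
; On BeginPlay it launches along local negative Z via ProjectileMovement and destroys itself after a fixed delay.
; Stripe overlap begin and end play timelines driving the mesh's ColorMultiplier material parameter.
; On exit, if IsDestroyed is true, a separate timeline also animates mesh scale; nothing here sets that flag true.
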(event EventBeginPlay
  (Variables|Default|SetIsDestroyed? false)
  (Game|Components|ProjectileMovement|SetVelocityinLocalSpace (Variables|Default|GetProjectileMovement) "0.000000,0.000000,-2000.000000")
  (Utilities|FlowControl|Delay 3.0)
  (Actor|DestroyActor))

(event Collision|EventActorBeginOverlap
  (params (OtherActor :type Actor%20Object%20Reference))
  (Utilities|Casting|CastToBP_TargetStripe OtherActor)
  (bind _colormultipliertrack (Timeline|Timeline Play)
    (:Update
      (Rendering|Material|SetScalarParameterValueonMaterials (Variables|Debug|GetStaticMeshComponent) "ColorMultiplier" _colormultipliertrack))))

(event Collision|EventActorEndOverlap
  (params (OtherActor :type Actor%20Object%20Reference))
  (bind _staticmeshcomponent (Variables|Debug|GetStaticMeshComponent))
  (Utilities|Casting|CastToBP_TargetStripe OtherActor)
  (if (not (Variables|Default|GetIsDestroyed?))
    (bind _colormultipliertrack (Timeline|Timeline_0 Play)
      (:Update
        (Rendering|Material|SetScalarParameterValueonMaterials _staticmeshcomponent "ColorMultiplier" _colormultipliertrack)))
    (else
      (bind (_direction _meshsizetrack _colormultipliertrack_2) (Timeline|Timeline_1 Play)
        (:Update
          (Transformation|SetRelativeScale3D _staticmeshcomponent (* (Math|Conversions|ToVector(Float) _meshsizetrack) (Math|Conversions|ToVector(Float) 4.44)))
          (Rendering|Material|SetScalarParameterValueonMaterials _staticmeshcomponent "ColorMultiplier" _colormultipliertrack_2))))))

(fn ConstructionScript)