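; Rhythm controller that plays a song and spawns colored target spheres in time with the song-specific Beat data table, announcing song start and completion.
; Audio playback percent sets elapsed time, and Tick processes at most one due table row per frame, using an event counter as row name.
; SpawnTarget re-reads the spawn site location and ship platform rotation, picks an arrow sphere class by color string, then tints and tags it.
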(event Custom|SpawnTarget
  (params (Color :type String))
  ;[0.15 0.15 0.15 0.5] Spawn target sphere at spawn location with color specified in Beat data table
  (CallFunction|GetLocations)
  (bind _target_sphere_reference (CallFunction|SpawnTargetSphere (Math|Transform|MakeTransform (Variables|Default|GetSpawnWorldLocation) (Variables|Default|GetShipRotation)) Color))
  (bind _color (CallFunction|GetColor Color))
  (Rendering|Material|SetVectorParameterValueonMaterials (Variables|/Game/Blueprints/BP_TargetSphere_Arrow.BP_TargetSphere_Arrow_C|GetStaticMesh_TriangularPrism _target_sphere_reference) "Color" (Math|Conversions|ToVector(LinearColor) _color))
  (Rendering|Material|SetScalarParameterValueonMaterials (Variables|/Game/Blueprints/BP_TargetSphere_Arrow.BP_TargetSphere_Arrow_C|GetStaticMesh_TriangularPrism _target_sphere_reference) "ColorMultiplier" 5.0)
  (Variables|/Script/Engine.Actor|SetTags _target_sphere_reference (Utilities|Array|MakeArray (Utilities|String|StringToName Color))))

(event Custom|GetLocations
  ;[0.15 0.15 0.15 0.5] Get location to spawn target spheres
  (bind _returnvalue (Actor|GetActorOfClass "/Game/VRTemplate/Blueprints/BP_SpawnSite.BP_SpawnSite_C"))
  (Utilities|IsValid _returnvalue
    (:Is%20Valid
      (Variables|Default|SetSpawnWorldLocation (Transformation|GetWorldLocation (Variables|/Script/Engine.Actor|GetRootComponent _returnvalue)))
      (bind _returnvalue_2 (Actor|GetActorOfClass "/Game/Scripting/BP_ShipPlatform.BP_ShipPlatform_C"))
      (Variables|Default|SetShipRotation (Transformation|GetWorldRotation (Variables|/Script/Engine.StaticMeshActor|GetStaticMeshComponent _returnvalue_2)))
      (Variables|Default|SetShipPlatform _returnvalue_2))))

(event Custom|SetAudioTimer
  (params (PlayingSoundWave :type Sound%20Wave%20Object%20Reference) (PlaybackPercent :type Float%20%28single-precision%29))
  (Variables|Default|SetSongTimeElapsed (* (Variables|Default|GetSongDuration) PlaybackPercent)))

(event Custom|OnAudioFinished_Event
  (Default|CallSongComplete))

(event EventTick
  (params (DeltaSeconds :type Float%20%28single-precision%29))
  (bind _eventcount (Variables|Default|GetEventCount))
  ;[0.15 0.15 0.15 0.5] Spawn target spheres when time has elapsed that matches time values in Beat data table (song-specific)
  (bind _returnvalue (Utilities|GetDataTableRow (Variables|Default|GetBeat) (Utilities|String|StringToName (Utilities|String|ToString(Integer) _eventcount)))
    (:then
      (if (<= (.Time (Utilities|Struct|BreakBP_BeatEvent _returnvalue)) (Variables|Default|GetSongTimeElapsed))
        (Math|Integer|IncrementInt _eventcount
          (:%20%20
            (if (Utilities|Enum|Equal(Enum) (.EventType (Utilities|Struct|BreakBP_BeatEvent _returnvalue)) "SpawnTarget")
              (CallFunction|SpawnTarget (.Param (Utilities|Struct|BreakBP_BeatEvent _returnvalue))))))))))

(event EventBeginPlay
  (Utilities|FlowControl|Delay 0.05)
  (bind _output_get (Variables|Default|SetSongTrack (Variables|Default|GetCosmic_Shores_WIP_20250817)))
  (Variables|Default|SetSongDuration (Variables|/Script/Engine.SoundBase|GetDuration (Variables|/Script/Engine.AudioComponent|GetSound _output_get)))
  (CallFunction|GetLocations)
  (EventDispatchers|BindEventtoOnAudioPlaybackPercent _output_get (delegate Custom|SetAudioTimer))
  (Variables|Default|SetEventCount 0)
  (Variables|Default|SetSongTimeElapsed 0.0)
  (Audio|Components|Audio|Play _output_get 0.0)
  (Default|CallSongStarted (Variables|Default|GetSongDuration))
  (EventDispatchers|AssignOnAudioFinished _output_get (delegate Custom|OnAudioFinished_Event)))

(fn ConstructionScript)

(fn SpawnTargetSphere
  (params (Spawn%20Transform :type Transform) (Color%20String :type String))
  (switch string Color%20String
    (:Default
      _)
    (:White
      _)
    (:Green
      (bind _returnvalue (Game|SpawnActorfromClass "/Game/Blueprints/BP_TargetSphere_GreenArrow.BP_TargetSphere_GreenArrow_C" Spawn%20Transform "Undefined" "MultiplyWithRoot" 0 0))
      (return _returnvalue))
    (:Red
      (bind _returnvalue_2 (Game|SpawnActorfromClass "/Game/Blueprints/BP_TargetSphere_RedArrow.BP_TargetSphere_RedArrow_C" Spawn%20Transform "Undefined" "MultiplyWithRoot" 0 0))
      (return _returnvalue_2))
    (:Blue
      (bind _returnvalue_3 (Game|SpawnActorfromClass "/Game/Blueprints/BP_TargetSphere_BlueArrow.BP_TargetSphere_BlueArrow_C" Spawn%20Transform "Undefined" "MultiplyWithRoot" 0 0))
      (return _returnvalue_3))
    (:Yellow
      (bind _returnvalue_4 (Game|SpawnActorfromClass "/Game/Blueprints/BP_TargetSphere_YellowArrow.BP_TargetSphere_YellowArrow_C" Spawn%20Transform "Undefined" "MultiplyWithRoot" 0 0))
      (return _returnvalue_4)))
  (bind _returnvalue_5 (Game|SpawnActorfromClass "/Game/Blueprints/BP_TargetSphere_WhiteArrow.BP_TargetSphere_WhiteArrow_C" Spawn%20Transform "Undefined" "MultiplyWithRoot" 0 0))
  (return _returnvalue_5))

(fn GetColor
  (params (ColorString :type String))
  (switch string ColorString
    (:Default
      _)
    (:White
      _)
    (:Green
      (return "(R=0.000000,G=1.000000,B=0.000000,A=1.000000)"))
    (:Red
      (return "(R=1.000000,G=0.000000,B=0.000000,A=1.000000)"))
    (:Blue
      (return "(R=0.000000,G=0.000000,B=1.000000,A=1.000000)"))
    (:Yellow
      (return "(R=0.800000,G=0.800000,B=0.000000,A=1.000000)")))
  (return "(R=0.411000,G=0.411000,B=0.411000,A=1.000000)"))