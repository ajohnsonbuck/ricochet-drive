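; BP_ShipMovement rotates the skybox, Earth sphere and ship platform over the course of a song, following a data-table program.
; BP_BeatController's song events start and stop it, while Tick advances completion as a fraction of song length.
; Each frame, rows matched by actor tag add rotation deltas, scaled by stretched half-sine or sigmoid-derivative rate curves.
; MoveActorByDelta applies only rotation; its translation inputs are unused.
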(event Custom|EndMovementProgram
  (Variables|Default|SetIsSongComplete? true))

(event Custom|SetMovementProgram
  (params (SongLength :type Float%20%28double-precision%29))
  (Variables|Default|SetSongLength SongLength)
  (bind _outrownames (DataTable|GetDataTableRowNames (Variables|Default|GetMovementProgram)))
  (Variables|Default|SetMovementProgramRows _outrownames)
  (bind _returnvalue (Actor|GetActorOfClass "/Game/Blueprints/BP_Skybox.BP_Skybox_C"))
  (bind _returnvalue_2 (Actor|GetActorOfClass "/Game/_GENERATED/BP_EarthSphere.BP_EarthSphere_C"))
  (bind _returnvalue_3 (Actor|GetActorOfClass "/Game/Scripting/BP_ShipPlatform.BP_ShipPlatform_C"))
  (Variables|Default|SetMovingActors (Utilities|Array|MakeArray _returnvalue _returnvalue_2 _returnvalue_3))
  (Variables|Default|SetIsSongStarted? true))

(event EventBeginPlay
  (bind _returnvalue (Actor|GetActorOfClass "/Game/Scripting/BP_ShipPlatform.BP_ShipPlatform_C"))
  (Variables|Default|SetShip _returnvalue)
  (bind _returnvalue_2 (Actor|GetActorOfClass "/Game/Blueprints/BP_BeatController.BP_BeatController_C"))
  (EventDispatchers|BindEventtoSongStarted _returnvalue_2 (delegate Custom|SetMovementProgram))
  (EventDispatchers|BindEventtoSongComplete _returnvalue_2 (delegate Custom|EndMovementProgram)))

(event EventTick
  (params (DeltaSeconds :type Float%20%28single-precision%29))
  (bind _songlength (Variables|Default|GetSongLength))
  (bind _returnvalue (/ DeltaSeconds _songlength))
  (if (and (Variables|Default|GetIsSongStarted?) (not (Variables|Default|GetIsSongComplete?)))
    (bind _output_get (Variables|Default|SetFractionStageComplete (+ (Variables|Default|GetFractionStageComplete) _returnvalue)))
    (for _array_element (Variables|Default|GetMovementProgramRows)
      (bind _returnvalue_2 (Utilities|GetDataTableRow (Variables|Default|GetMovementProgram) _array_element)
        (:then
          (for _array_element_2 (Variables|Default|GetMovingActors)
            (if (Actor|ActorHasTag _array_element_2 (.Actor (Utilities|Struct|BreakMovementProgram _returnvalue_2)))
              (bind _deltatrajectory (CallFunction|FractionComplete2Trajectory _output_get (.TimeFunction (Utilities|Struct|BreakMovementProgram _returnvalue_2)) (.Param1 (Utilities|Struct|BreakMovementProgram _returnvalue_2)) (.Param2 (Utilities|Struct|BreakMovementProgram _returnvalue_2))))
              (CallFunction|MoveActorbyDelta _array_element_2 0.0 0.0 0.0 (* (* _deltatrajectory _returnvalue) (.deltaXrot (Utilities|Struct|BreakMovementProgram _returnvalue_2))) (* (* _deltatrajectory _returnvalue) (.deltaYrot (Utilities|Struct|BreakMovementProgram _returnvalue_2))) (* (* _deltatrajectory _returnvalue) (.deltaZrot (Utilities|Struct|BreakMovementProgram _returnvalue_2)))))))))))

(fn ConstructionScript)

(fn FractionComplete2Trajectory
  (params (FractionStageComplete :type Float%20%28double-precision%29) (TimeFunction :type String) (Param1 :type Float%20%28double-precision%29) (Param2 :type Float%20%28double-precision%29))
  (if (Utilities|Enum|Equal(Enum) TimeFunction "StretchedSine")
    (bind _returnvalue (Class|RicochetDriveMathFunctionLibrary|StretchedHalfSine FractionStageComplete Param1 Param2))
    (return _returnvalue)
    (elif (Utilities|Enum|Equal(Enum) TimeFunction "CompressedSigmoid")
      (bind _returnvalue_2 (Class|RicochetDriveMathFunctionLibrary|CompressedSigmoidalDiff FractionStageComplete Param1 Param2))
      (return _returnvalue_2))))

(fn MoveActorbyDelta
  (params (Actor :type Actor%20Object%20Reference) (deltaX :type Float%20%28double-precision%29) (deltaY :type Float%20%28double-precision%29) (deltaZ :type Float%20%28double-precision%29) (deltaXrot :type Float%20%28double-precision%29) (deltaYrot :type Float%20%28double-precision%29) (deltaZrot :type Float%20%28double-precision%29))
  (bind _rootcomponent (Variables|/Script/Engine.Actor|GetRootComponent Actor))
  (bind _relativerotation (Variables|/Script/Engine.SceneComponent|GetRelativeRotation _rootcomponent))
  (Transformation|SetRelativeRotation _rootcomponent (Math|Rotator|MakeRotator (+ deltaXrot (.roll _relativerotation)) (+ deltaYrot (.pitch _relativerotation)) (+ deltaZrot (.yaw _relativerotation))) false false))