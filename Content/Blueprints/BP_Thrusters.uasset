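; BP_Thrusters drives the Niagara engine exhaust on BP_Engine, reflecting the player's combo score.
; UpdateThrusters stretches the sprites with score, using thresholds and colors from BP_ScoreKeeper.
; Hitting a threshold above one briefly hides the flame, then plays a score-scaled sound, two-hand haptics, color change and timeline size boost, bracketed by boost dispatchers.
; The final combo level spawns an additional plaid thruster system, destroyed on returning to lower levels.
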(event Custom|UpdateThrusters
  (params (Combo%20Score :type Integer))
  (bind _combothresholds (Variables|Default|GetComboThresholds))
  (bind _returnvalue (Utilities|Array|FindItem _combothresholds Combo%20Score))
  ;[0.15 0.15 0.15 0.5] Use Combo Score to Update Thruster Color and Size
  (bind _sprite_size (CallFunction|CalculateThrusterParameters Combo%20Score))
  (Class|NiagaraComponent|SetNiagaraVariableVec2 (Variables|Default|GetThruster) "Sprite Size" _sprite_size)
  (if (and (!= Combo%20Score 1) (!= _returnvalue -1))
    (CallFunction|ThrusterLevelUp Combo%20Score _returnvalue _sprite_size)
    (elif (<= Combo%20Score 1)
      (CallFunction|SetThrusterColor))))

(event Custom|Thruster%20Level%20Up
  (params (Combo%20Score :type Integer) (Combo%20Level :type Integer) (Starting%20Sprite%20Size :type Vector%202D%20Structure))
  (bind _returnvalue (Game|GetPlayerController 0))
  ;[0.15 0.15 0.15 0.5] Play Sound and Rumble on Reaching a New Combo Level
  (Default|CallThrusterBoostActive)
  (Class|NiagaraComponent|SetNiagaraVariableVec2 (Variables|Default|GetThruster) "Sprite Size")
  (Utilities|FlowControl|Delay 0.5)
  (Audio|PlaySoundatLocation "/Game/SFX/366088__bevibeldesign__huge-explosion-part-2-impact.366088__bevibeldesign__huge-explosion-part-2-impact" (Transformation|GetWorldLocation (Variables|Default|GetDefaultSceneRoot)) "0, 0, 0" (Math|Float|Lerp 0.75 1.25 (/ (Math|Conversions|ToFloat(Integer) Combo%20Score) (Math|Conversions|ToFloat(Integer) (.MaxValue (Math|Integer|MaxOfIntArray (Variables|Default|GetComboThresholds)))))) 1.0 0.0 0 0 0 0)
  (Class|PlayerController|PlayHapticEffect _returnvalue "/Game/VRTemplate/Haptics/ThrusterLow.ThrusterLow" "Left" 1.0 false)
  (Class|PlayerController|PlayHapticEffect _returnvalue "/Game/VRTemplate/Haptics/ThrusterLow.ThrusterLow" "Right" 1.0 false)
  (CallFunction|SetThrusterColor Combo%20Level)
  (bind _spritesizemultiplier (Timeline|ThrusterBoost PlayFromStart)
    (:Update
      (Class|NiagaraComponent|SetNiagaraVariableVec2 (Variables|Default|GetThruster) "Sprite Size" (* Starting%20Sprite%20Size (Math|Vector2D|MakeVector2D 1.0 _spritesizemultiplier))))
    (:Finished
      (Default|CallThrusterBoostStopped))))

(event Custom|Set%20Thruster%20Color
  (params (Combo%20Level :type Integer))
  (bind _combocolors (Variables|Default|GetComboColors))
  (bind _thruster (Variables|Default|GetThruster))
  (bind _plaidthruster (Variables|Default|GetPlaidThruster))
  ;[0.15 0.15 0.15 0.5] Set Thruster Color (Excludes Plaid Mode)
  (if (< Combo%20Level (- (Utilities|Array|Length _combocolors) 1))
    (Effects|Components|ParticleSystem|SetColorParameter _thruster "Linear Color" (.SpecifiedColor (Utilities|Struct|BreakSlateColor (Utilities|Array|Get(acopy) _combocolors Combo%20Level))))
    (Variables|Default|SetGoneToPlaid false)
    (if (Utilities|IsValid _plaidthruster)
      (Components|DestroyComponent _plaidthruster))
    (elif (not (Variables|Default|GetGoneToPlaid))
      (CallFunction|GotoPlaid _thruster))))

(event Custom|Go%20To%20Plaid
  (params (Thruster :type Niagara%20Component%20Object%20Reference))
  ;[0.15 0.15 0.15 0.5] Set thrusters to plaid
  (bind _returnvalue (Niagara|SpawnSystematLocation "/Game/VFX/NS_PlaidThruster.NS_PlaidThruster" (+ (Transformation|GetWorldLocation Thruster) (Math|Vector|MakeVector 0.0 0.0 -5e+03))))
  (Variables|Default|SetPlaidThruster _returnvalue)
  (Variables|Default|SetGoneToPlaid true))

(event EventBeginPlay
  (bind _returnvalue (Actor|GetActorOfClass "/Game/Blueprints/BP_Engine.BP_Engine_C"))
  (bind _returnvalue_2 (Niagara|SpawnSystemAttached "/Game/VFX/NS_Thruster.NS_Thruster" (Variables|/Script/Engine.Actor|GetRootComponent _returnvalue) "None" "0.000000,-4500.000000,0.000000" "0, 0, 0" "KeepRelativeOffset" false))
  (Niagara|SetNiagaraVariable(Float) _returnvalue_2 "Radius" 1.2e+03)
  (Variables|Default|SetThruster _returnvalue_2)
  ;[0.15 0.15 0.15 0.5] Get Combo Thresholds from BP_Scorekeeper
  (bind _returnvalue_3 (Actor|GetActorOfClass "/Game/Blueprints/BP_ScoreKeeper.BP_ScoreKeeper_C"))
  (Variables|Default|SetComboThresholds (Variables|/Game/Blueprints/BP_ScoreKeeper.BP_ScoreKeeper_C|GetComboThresholds _returnvalue_3))
  (Variables|Default|SetComboColors (Variables|/Game/Blueprints/BP_ScoreKeeper.BP_ScoreKeeper_C|GetComboColors _returnvalue_3))
  (CallFunction|UpdateThrusters (Variables|/Game/Blueprints/BP_ScoreKeeper.BP_ScoreKeeper_C|GetComboScore _returnvalue_3)))

(fn ConstructionScript)

(fn CalculateThrusterParameters
  (params (ComboScore :type Integer))
  (bind _returnvalue (Math|Conversions|ToFloat(Integer) ComboScore))
  (return (+ (* _returnvalue 0.002) 1.0) (+ (* _returnvalue 0.005) 0.2) (Math|Vector2D|MakeVector2D 2.5e+02 (+ (* _returnvalue 2e+02) 3e+03))))