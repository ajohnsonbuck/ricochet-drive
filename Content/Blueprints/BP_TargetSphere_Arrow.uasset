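; BP_TargetSphere_Arrow is a laser target sphere with a colored arrow prism that counts as a hit or miss.
; Overlap with BP_TargetStripe toggles targetability and collision; leaving unhit reports a miss to BP_ScoreKeeper and sets the prism's ColorMultiplier from the never-played Darken timeline.
; A laser hit reports once, then timelines shrink the sphere, animate prism brightness and expand a temporary BP_ExplosionShell shockwave, colored from the first actor tag.
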(event Custom|HitByLaser
  ;[0.15 0.15 0.15 0.5] If hit by laser, set as destroyed, register as hit with Score Keeper, and shrink into tiny glowing ball
  (if (not (Variables|Default|GetIsDestroyed?))
    (Variables|Default|SetIsDestroyed? true)
    (bind _returnvalue (Actor|GetActorOfClass "/Game/Blueprints/BP_ScoreKeeper.BP_ScoreKeeper_C"))
    (Default|AddHit _returnvalue)
    (CallFunction|SpawnShockwave)
    (bind (_direction _meshsizetrack _colormultipliertrack) (Timeline|Brighten%20and%20shrink%20if%20hit Play)
      (:Update
        (Transformation|SetRelativeScale3D (Variables|Default|GetStaticMeshComponent) (Math|Conversions|ToVector(Float) _meshsizetrack))
        (Rendering|Material|SetScalarParameterValueonMaterials (Variables|Default|GetStaticMesh_TriangularPrism) "ColorMultiplier" _colormultipliertrack)))))

(event Custom|Spawn%20Shockwave
  ;[0.15 0.15 0.15 0.5] Spawn Shockwave on Hit By Correct  Laser
  (bind _returnvalue (Game|SpawnActorfromClass "/Game/Blueprints/BP_ExplosionShell.BP_ExplosionShell_C" (Math|Conversions|ToTransform(Vector) (Transformation|GetWorldLocation (Variables|Default|GetStaticMeshComponent))) "Undefined" "MultiplyWithRoot" 0 0))
  (bind _color (CallFunction|ParseColorfromTag (Utilities|Array|Get(acopy) (Variables|Default|GetTags self))))
  (Rendering|Material|SetVectorParameterValueonMaterials (Variables|/Game/Blueprints/BP_ExplosionShell.BP_ExplosionShell_C|GetSphere _returnvalue) "Color" _color)
  (bind (_direction _scale _opacity) (Timeline|ShellExpansion Play)
    (:Update
      (Transformation|SetRelativeScale3D (Variables|/Game/Blueprints/BP_ExplosionShell.BP_ExplosionShell_C|GetSphere _returnvalue) (Math|Conversions|ToVector(Float) _scale))
      (Rendering|Material|SetScalarParameterValueonMaterials (Variables|/Game/Blueprints/BP_ExplosionShell.BP_ExplosionShell_C|GetSphere _returnvalue) "OpacityMultiplier" _opacity))
    (:Finished
      (Actor|DestroyActor _returnvalue))))

(event Collision|EventActorBeginOverlap
  (params (OtherActor :type Actor%20Object%20Reference))
  ;[0.15 0.15 0.15 0.5] Set as targetable once entering target zone (mainly matters for non-VR debug mode)
  (Utilities|Casting|CastToBP_TargetStripe OtherActor)
  (Variables|Default|SetIsTargetable true)
  (Collision|SetCollisionEnabled (Variables|Default|GetStaticMeshComponent) "QueryAndPhysics"))

(event Collision|EventActorEndOverlap
  (params (OtherActor :type Actor%20Object%20Reference))
  ;[0.15 0.15 0.15 0.5] Once leaving target zone, set as not targetable.  If not destroyed, register as miss and dim colored part of sphere.
  (Utilities|Casting|CastToBP_TargetStripe OtherActor)
  (Variables|Default|SetIsTargetable false)
  (Collision|SetCollisionEnabled (Variables|Default|GetStaticMeshComponent) "NoCollision")
  (if (not (Variables|Default|GetIsDestroyed?))
    (bind _returnvalue (Actor|GetActorOfClass "/Game/Blueprints/BP_ScoreKeeper.BP_ScoreKeeper_C"))
    (Default|AddMiss _returnvalue)
    (Rendering|Material|SetScalarParameterValueonMaterials (Variables|Default|GetStaticMesh_TriangularPrism) "ColorMultiplier" (stale _colormultipliertrack))))

(fn ConstructionScript
  (|CallParentFunction))

(fn ParseColorfromTag
  (params (ColorTag :type Name))
  (if (== ColorTag (Utilities|Name|MakeLiteralName "Red"))
    (return (Math|Conversions|ToVector(LinearColor) (Utilities|Struct|MakeLinearColor 1.0 0.0 0.0 0.0)))
    (elif (== ColorTag (Utilities|Name|MakeLiteralName "Blue"))
      (return (Math|Conversions|ToVector(LinearColor) (Utilities|Struct|MakeLinearColor 0.0 0.0 1.0 0.0)))
      (elif (== ColorTag (Utilities|Name|MakeLiteralName "Green"))
        (return (Math|Conversions|ToVector(LinearColor) (Utilities|Struct|MakeLinearColor 0.0 1.0 0.0 0.0)))
        (elif (== ColorTag (Utilities|Name|MakeLiteralName "Yellow"))
          (return (Math|Conversions|ToVector(LinearColor) (Utilities|Struct|MakeLinearColor 1.0 1.0 0.0 0.0)))
          (elif (== ColorTag (Utilities|Name|MakeLiteralName "White"))
            (return (Math|Conversions|ToVector(LinearColor) (Utilities|Struct|MakeLinearColor 1.0 1.0 1.0 0.0)))))))))