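; BP_Sunlight is an actor that keeps its rotation aimed along the direction from the BP_Sun actor to the player, so sunlight appears to come from the sun.
; At BeginPlay it finds BP_Sun in the level and starts a short looping timer instead of using Tick.
; Each timer call builds a rotation from the unit vector between the sun's mesh and the player pawn and applies it to itself.
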(event Custom|UpdateLightRotation
  (Transformation|SetActorRotation (Math|Conversions|RotationFromXVector (Math|Vector|GetUnitDirection(Vector) (Transformation|GetWorldLocation (Variables|/Script/Engine.StaticMeshActor|GetStaticMeshComponent (Variables|Default|GetSun))) (Transformation|GetActorLocation (Game|Player|GetPlayerPawn 0))))))

(event EventBeginPlay
  (bind _returnvalue (Actor|GetActorOfClass "/Game/Materials/BP_Sun.BP_Sun_C"))
  (Variables|Default|SetSun _returnvalue)
  (Utilities|Time|SetTimerbyEvent (delegate Custom|UpdateLightRotation) 0.1 true))

(fn ConstructionScript)